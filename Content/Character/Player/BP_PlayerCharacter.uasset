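; Player character Blueprint for melee combat with twin blades, avoidance, damage and death, plus a parameter HUD.
; Attack and avoid inputs drive BP_PlayerAnim, whose events reset action states; attacking during avoidance becomes a dash attack.
; Combo events toggle blade collision, and hits deal defence-based damage, spawn effects and trigger hit stop through time dilation.
; Avoidance spawns BP_Avoid actors each tick, while a timeline drains HP and death ends in ragdoll.
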(event `DamageCancel`
  ;[1 1 1] ダメージ処理の中止
  (set `self.Damaging` false))

(event `Attackcancel`
  ;[1 1 1] 攻撃中止
  (set `self.Attacking` false))

(event `self.ReceiveBeginPlay`
  ;[1 1 1] 初期化
  (bind _asbp_player_anim (cast `/Game/Character/Animation/SwordCharacter/Player/BP_PlayerAnim` (`SkeletalMeshComponent.GetAnimInstance` (`self.Mesh`))))
  (bind _output_get (set `self.MyAnim` _asbp_player_anim))
  (add `/Game/Character/Animation/SwordCharacter/Player/BP_PlayerAnim.CharacterDeath` _output_get (delegate `self.PlayerDeath`))
  (add `/Game/Character/Animation/SwordCharacter/Player/BP_PlayerAnim.AttackCancel` _output_get (delegate `Attackcancel`))
  (add `/Game/Character/Animation/SwordCharacter/Player/BP_PlayerAnim.DamageCancel` _output_get (delegate `DamageCancel`))
  (add `/Game/Character/Animation/SwordCharacter/Player/BP_PlayerAnim.ComboEnd` _output_get (delegate `AttackEnd`))
  (add `self.PlayerCombo` (delegate `SetCollision`))
  (add `self.CollisionEnd` (delegate `SetUnCollision`))
  (add `self.OnHitStop` (delegate `HitStopEvent`))
  (`self.InitializeStatus` 0)
  (bind _returnvalue (`|CreateWidget` "/Game/Character/Player/Widget/UI_PlayerParam.UI_PlayerParam_C"))
  (set `/Game/Character/Widget/UI_CharacterMaster.PlayerCharacter` self _returnvalue)
  (`UserWidget.AddToViewport` _returnvalue 0))

(event `self.PlayerDeath`
  ;[1 1 1] 死亡処理
  (`SkeletalMeshComponent.SetAllBodiesSimulatePhysics` (`self.Mesh`) true))

(event `HitStopEvent`
  ;[1 1 1] ヒットストップ
  (`self.HitStop` self 0.5 0.25))

(event `AttackEnd`
  ;[1 1 1] 攻撃終了
  (bind _output_get (set `self.Attacking` false))
  (`self.CheckFlyAttack` _output_get)
  (`self.CollisionEnd`))

(event `SetUnCollision`
  ;[1 1 1] コリジョンの設定(無効化)
  (`self.UnUseCollision` (`self.RightBlade`) (`self.LeftBlade`)))

(event `SetCollision` :!signature `self.PlayerCombo`
  (params (ComboCount :type Integer))
  (bind _rightblade (`self.RightBlade`))
  (bind _leftblade (`self.LeftBlade`))
  ;[1 1 1] コリジョンの設定(有効化)
  (switch `int` ComboCount
    (:`0`
      (`self.UseCollision` _rightblade))
    (:`1`
      (`self.UseCollision` _leftblade))
    (:`2`
      (`self.UseCollision` _leftblade)
      (`self.UseCollision` _rightblade))))

(event `InputAction|Attack`
  (params (Key :type "Key Structure"))
  (bind _myanim (`self.MyAnim`))
  ;[1 1 1] 攻撃イベント
  (:`Pressed`
    (if (and (not (`/Game/Character/Animation/SwordCharacter/Player/BP_PlayerAnim.IsCombo` (`self.MyAnim`))) (`self.Attacking`))
      _
      (elif (`self.Avoiding`)
        (`/Game/Character/Animation/SwordCharacter/Player/BP_PlayerAnim.DashAttackEvent` _myanim)
        (`self.AvoidCancel`)
        (bind _output_get (set `self.Attacking` true))
        (`self.CheckFlyAttack` _output_get)
        (else
          (`/Game/Character/Animation/SwordCharacter/Player/BP_PlayerAnim.AttackEvent` _myanim)
          (bind _output_get_2 (set `self.Attacking` true))
          (`self.CheckFlyAttack` _output_get_2))))))

(event `self.RightBlade.OnComponentBeginOverlap`
  (params (OverlappedComponent :type "PrimitiveComponent Object Reference") (OtherActor :type "Actor Object Reference") (OtherComp :type "PrimitiveComponent Object Reference") (OtherBodyIndex :type Integer) (bFromSweep :type Boolean) (SweepResult :type "HitResult Structure (by ref)"))
  ;[1 1 1] 攻撃判定
  (bind _asenemy_character (cast `EnemyCharacter` OtherActor))
  (if (!= _asenemy_character self)
    (bind (_myparam_id _myparam_name _myparam_maxhp _myparam_power _myparam_defence) (break `CharacterStatus` (`EnemyCharacter.MyParam` _asenemy_character)))
    (`self.GiveDamage` _asenemy_character _myparam_defence)
    (bind _returnvalue (`|SpawnActorFromClass` "/Game/Effect/BP_AttackEffect.BP_AttackEffect_C" (`SceneComponent.K2_GetComponentToWorld` OverlappedComponent) "Undefined" "OverrideRootScale" null null))
    (`self.OnHitStop`)
    (`self.HitStop` _returnvalue 0.5 0.25)))

(event `self.ReceiveTick`
  (params (DeltaSeconds :type "Float (single-precision)"))
  ;[1 1 1] 更新処理
  (`|ExecutionSequence`
    (:`then_0`
      (`/Engine/EditorBlueprintResources/StandardMacros.DoOnce` false
        (:`Completed`
          (`self.InputInitialize`))))
    (:`then_1`
      (if (`self.Avoiding`)
        (`KismetSystemLibrary.Delay` 0.02)
        (bind _returnvalue (`|SpawnActorFromClass` "/Game/Effect/BP_Avoid.BP_Avoid_C" (`self.GetTransform`) "Undefined" "OverrideRootScale" null null))
        (`/Game/Effect/BP_Avoid.SetOpacity` _returnvalue (`self.PlayerOrigin`))))))

(event `self.LeftBlade.OnComponentBeginOverlap`
  (params (OverlappedComponent :type "PrimitiveComponent Object Reference") (OtherActor :type "Actor Object Reference") (OtherComp :type "PrimitiveComponent Object Reference") (OtherBodyIndex :type Integer) (bFromSweep :type Boolean) (SweepResult :type "HitResult Structure (by ref)"))
  ;[1 1 1] 攻撃判定
  (bind _asenemy_character (cast `EnemyCharacter` OtherActor))
  (if (!= _asenemy_character self)
    (bind (_myparam_id _myparam_name _myparam_maxhp _myparam_power _myparam_defence) (break `CharacterStatus` (`EnemyCharacter.MyParam` _asenemy_character)))
    (`self.GiveDamage` _asenemy_character _myparam_defence)
    (bind _returnvalue (`|SpawnActorFromClass` "/Game/Effect/BP_AttackEffect.BP_AttackEffect_C" (`SceneComponent.K2_GetComponentToWorld` OverlappedComponent) "Undefined" "OverrideRootScale" null null))
    (`self.OnHitStop`)
    (`self.HitStop` _returnvalue 0.5 0.25)))

(event `InputAction|Avoid`
  (params (Key :type "Key Structure"))
  ;[1 1 1] 回避行動
  (:`Pressed`
    (if (not (`self.Avoiding`))
      (`/Game/Character/Animation/SwordCharacter/Player/BP_PlayerAnim.AvoidEvent` (`self.MyAnim`))
      (`self.AvoidAction`)
      (set `self.PlayerOrigin` (`self.K2_GetActorLocation`)))))

(event `self.ReceiveAnyDamage`
  (params (Damage :type "Float (single-precision)") (DamageType :type "DamageType Object Reference") (InstigatedBy :type "Controller Object Reference") (DamageCauser :type "Actor Object Reference"))
  (bind _returnvalue (- (`self.TotalDamage`) Damage))
  ;[1 1 1] ダメージ処理
  (bind _output_get (set `self.TotalDamage` (`self.HP`)))
  (if (<= _returnvalue 0.0)
    (bind (_direction _deltatime) (`Timeline|DamageValue` :!via `PlayFromStart` :!label _label)
      (:`Update`
        (bind _output_get_2 (set `self.HP` (`KismetMathLibrary.Lerp` _output_get _returnvalue _deltatime)))
        (if (<= _output_get_2 0.0)
          (`/Engine/EditorBlueprintResources/StandardMacros.DoOnce` false
            (:`Completed`
              (set `self.IsDeath` true)
              (`/Game/Character/Animation/SwordCharacter/Player/BP_PlayerAnim.DeathEvent` (`self.MyAnim`)))))))
    (else
      (`/Game/Character/Animation/SwordCharacter/Player/BP_PlayerAnim.DamageEvent` (`self.MyAnim`))
      (goto _label :!via `PlayFromStart`))))

(fn `UserConstructionScript`
  (`parent.UserConstructionScript`))