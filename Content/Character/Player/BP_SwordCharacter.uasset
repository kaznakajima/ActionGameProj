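; Player sword character Blueprint with helper graphs for stats, gamepad input, UI visibility, enemy search and hit stop.
; InitializeStatus loads HP and parameters from the MyCharacterData table by row name, while InputInitialize remaps A/B for PS4 controllers through DirectInput.
; GetMinDistanceEnemy scans all EnemyCharacter actors for the nearest one.
; HitStop briefly changes a given actor's CustomTimeDilation, then restores it to normal after a delay.
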(fn `GetMinDistanceEnemy`
  (returns (ReturnValue :type "EnemyCharacter Object Reference"))
  (locals (MinDistance :type "Float (double-precision)") (returnActor :type "EnemyCharacter Object Reference"))
  (bind _mindistance (`local.MinDistance`))
  ;[1 1 1] 一番近い敵を返す
  (bind _outactors (`GameplayStatics.GetAllActorsOfClass` "/Script/ActionGame.EnemyCharacter"))
  (for _array_element _outactors
    (bind _returnvalue (`self.GetDistanceTo` _array_element))
    (if (or (<= _returnvalue _mindistance) (== _mindistance 0.0))
      (set `local.MinDistance` _returnvalue)
      (set `local.returnActor` _array_element)))
  (set `local.MinDistance` 0.0)
  (return (`local.returnActor`)))

(fn `InitializeStatus`
  (params (Name :type Name))
  (locals (NewLocalVar_0 :type " Structure"))
  ;[1 1 1] ステータス初期化
  (bind _outrownames (`DataTableFunctionLibrary.GetDataTableRowNames` "/Game/Character/MyCharacterData.MyCharacterData"))
  (for _array_element _outrownames
    (if (== _array_element Name)
      (bind _returnvalue (`|GetDataTableRow` "/Game/Character/MyCharacterData.MyCharacterData" _array_element)
        (:`then`
          (set `self.HP` (`.MaxHP` (break `MyData` _returnvalue)))
          (set `self.MyParam` (make `CharacterStatus` (break `MyData` _returnvalue) (`.Name` (break `MyData` _returnvalue)) (`.MaxHP` (break `MyData` _returnvalue)) (`.Power` (break `MyData` _returnvalue)) (`.Defence` (break `MyData` _returnvalue)))))))))

(fn `InputInitialize`
  (bind _returnvalue (`DirectInputPadFunctionLibrary.GetDirectInputPadJoystick` 0))
  ;[1 1 1] PS4コントローラーに対応させる
  (`/Engine/EditorBlueprintResources/StandardMacros.IsValid` _returnvalue
    (:`Is Valid`
      (`/Engine/EditorBlueprintResources/StandardMacros.DoOnce` false :!label _label
        (:`Completed`
          (`DirectInputPadJoystick.SetKeyMap` _returnvalue "XIGamePad_Button_A" "DIGamePad_Button2" false)
          (`DirectInputPadJoystick.SetKeyMap` _returnvalue "XIGamePad_Button_B" "DIGamePad_Button3" false))))
    (:`Is Not Valid`
      (goto _label :!via `Reset`))))

(fn `UI_Initialize`
  ;[1 1 1] UIの初期化
  (set `self.MyUI` null))

(fn `UI_Switch`
  (params (Value :type Boolean))
  ;[1 1 1] UIの表示非表示
  (if Value
    (`Widget.SetVisibility` (`self.MyUI`) "Hidden")
    (set `self.IsActive` false)
    (else
      (`Widget.SetVisibility` (`self.MyUI`) "Visible")
      (set `self.IsActive` true))))

(fn `UserConstructionScript`)