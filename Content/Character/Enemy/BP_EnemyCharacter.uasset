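; Enemy character with a two-blade combo attack and an avoid move, triggered by E and F keys.
; Combo events toggle blade collision; overlaps with BP_SwordCharacter deal damage, spawn effects and trigger hit stop through brief CustomTimeDilation slowdowns.
; Tick repositions the enemy's status widget and spawns BP_Avoid actors while avoiding.
; Incoming damage plays a reaction and drains HP over a timeline, removing the widget and actor at zero.
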(event `self.ReceiveBeginPlay`
  ;[1 1 1] 初期化
  (bind _asbp_player_anim (cast `/Game/Character/Animation/SwordCharacter/BP_PlayerAnim` (`SkeletalMeshComponent.GetAnimInstance` (`self.Mesh`))))
  (bind _output_get (set `self.MyAnim` _asbp_player_anim))
  (add `/Game/Character/Animation/SwordCharacter/BP_PlayerAnim.ComboEnd` _output_get (delegate `AttackEnd`))
  (add `self.PlayerCombo` (delegate `SetCollision`))
  (add `self.CollisionEnd` (delegate `SetUnCollision`))
  (add `self.P_HitStop` (delegate `HitStopEvent`))
  (`self.InitializeStatus` 1)
  (bind _returnvalue (`|CreateWidget` "/Game/Character/Enemy/Widget/UI_EnemyParam.UI_EnemyParam_C" (`GameplayStatics.GetPlayerController` 0)))
  (bind _output_get_2 (set `self.MyUI` _returnvalue))
  (set `/Game/Character/Widget/UI_CharacterMaster.MyCharacter` self _output_get_2)
  (`UserWidget.AddToViewport` _returnvalue 0))

(event `self.ReceiveTick`
  (params (DeltaSeconds :type "Float (single-precision)"))
  (bind _myui (`self.MyUI`))
  (`|ExecutionSequence`
    (:`then_1`
      (if (`KismetSystemLibrary.IsValid` _myui)
        (`/Game/Character/Widget/UI_CharacterMaster.SetUIPosition` _myui)))
    (:`then_2`
      (if (`self.Avoiding`)
        (`KismetSystemLibrary.Delay` 0.01)
        (bind _returnvalue (`|SpawnActorFromClass` "/Game/Effect/BP_Avoid.BP_Avoid_C" (`self.GetTransform`) "Undefined" "OverrideRootScale" null null))
        (`/Game/Effect/BP_Avoid.SetOpacity` _returnvalue (`self.PlayerOrigin`))))))

(event `AttackEnd`
  ;[1 1 1] 攻撃終了
  (set `self.Attacking` false)
  (`self.CollisionEnd`))

(event `HitStopEvent`
  ;[1 1 1] ヒットストップ
  (`self.HitStop` self 0.5 0.25))

(event `SetUnCollision`
  ;[1 1 1] コリジョンの設定(無効化)
  (`self.UnUseCollision` (`self.LeftBlade`) (`self.RightBlade`)))

(event `SetCollision` :!signature `self.PlayerCombo`
  (params (ComboCount :type Integer))
  ;[1 1 1] コリジョンの設定(有効化)
  (switch `int` ComboCount
    (:`0`
      (`self.UseCollision` (`self.RightBlade`)))
    (:`1`
      (`self.UseCollision` (`self.LeftBlade`)))))

(event `Key|E`
  (params (Key :type "Key Structure"))
  ;[1 1 1] 攻撃イベント
  (:`Pressed`
    (if (not (and (not (`/Game/Character/Animation/SwordCharacter/BP_PlayerAnim.IsCombo` (`self.MyAnim`))) (`self.Attacking`)))
      (`/Game/Character/Animation/SwordCharacter/BP_PlayerAnim.AttackEvent` (`self.MyAnim`))
      (set `self.Attacking` true))))

(event `self.RightBlade.OnComponentBeginOverlap`
  (params (OverlappedComponent :type "PrimitiveComponent Object Reference") (OtherActor :type "Actor Object Reference") (OtherComp :type "PrimitiveComponent Object Reference") (OtherBodyIndex :type Integer) (bFromSweep :type Boolean) (SweepResult :type "HitResult Structure (by ref)"))
  ;[1 1 1] 攻撃判定
  (bind _asbp_sword_character (cast `/Game/Character/BP_SwordCharacter` OtherActor))
  (bind (_myparam_id _myparam_name _myparam_maxhp _myparam_power _myparam_defence) (break `CharacterStatus` (`ActionGameCharacter.MyParam` _asbp_sword_character)))
  (`self.GiveDamage` _asbp_sword_character _myparam_defence)
  (bind _returnvalue (`|SpawnActorFromClass` "/Game/Effect/BP_AttackEffect.BP_AttackEffect_C" (`SceneComponent.K2_GetComponentToWorld` OverlappedComponent) "Undefined" "OverrideRootScale" null null))
  (`self.P_HitStop`)
  (`self.HitStop` _returnvalue 0.5 0.25))

(event `self.LeftBlade.OnComponentBeginOverlap`
  (params (OverlappedComponent :type "PrimitiveComponent Object Reference") (OtherActor :type "Actor Object Reference") (OtherComp :type "PrimitiveComponent Object Reference") (OtherBodyIndex :type Integer) (bFromSweep :type Boolean) (SweepResult :type "HitResult Structure (by ref)"))
  ;[1 1 1] 攻撃判定
  (bind _asbp_sword_character (cast `/Game/Character/BP_SwordCharacter` OtherActor))
  (bind (_myparam_id _myparam_name _myparam_maxhp _myparam_power _myparam_defence) (break `CharacterStatus` (`ActionGameCharacter.MyParam` _asbp_sword_character)))
  (`self.GiveDamage` _asbp_sword_character _myparam_defence)
  (bind _returnvalue (`|SpawnActorFromClass` "/Game/Effect/BP_AttackEffect.BP_AttackEffect_C" (`SceneComponent.K2_GetComponentToWorld` OverlappedComponent) "Undefined" "OverrideRootScale" null null))
  (`self.P_HitStop`)
  (`self.HitStop` _returnvalue 0.5 0.25))

(event `Key|F`
  (params (Key :type "Key Structure"))
  (:`Pressed`
    (`/Engine/EditorBlueprintResources/StandardMacros.DoOnce` false
      (:`Completed`
        (`/Game/Character/Animation/SwordCharacter/BP_PlayerAnim.AvoidEvent` (`self.MyAnim`))
        (`self.AvoidAction`)
        (set `self.PlayerOrigin` (`self.K2_GetActorLocation`))))))

(event `self.ReceiveAnyDamage`
  (params (Damage :type "Float (single-precision)") (DamageType :type "DamageType Object Reference") (InstigatedBy :type "Controller Object Reference") (DamageCauser :type "Actor Object Reference"))
  (bind _returnvalue (- (`self.TotalDamage`) Damage))
  ;[1 1 1] ダメージ処理
  (bind _output_get (set `self.TotalDamage` (`self.HP`)))
  (if (<= _returnvalue 0.0)
    _
    (else
      _))
  (`/Game/Character/Animation/SwordCharacter/BP_PlayerAnim.DamageEvent` (`self.MyAnim`))
  (bind (_direction _deltatime) (`Timeline|DamageValue` :!via `PlayFromStart`)
    (:`Update`
      (bind _output_get_2 (set `self.HP` (`KismetMathLibrary.Lerp` _output_get _returnvalue _deltatime)))
      (if (<= _output_get_2 0.0)
        (`Widget.RemoveFromParent` (`self.MyUI`))
        (`self.K2_DestroyActor`)))))

(fn `UserConstructionScript`
  (`parent.UserConstructionScript`))