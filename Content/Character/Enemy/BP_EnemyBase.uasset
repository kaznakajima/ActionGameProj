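; Base enemy character Blueprint that holds stats and helper routines for enemies.
; InitializeStatus picks the CharacterData row whose index matches the given ID, then sets HP to its max and fills MyParam.
; InputInitialize remaps the A and B buttons on DirectInput pad 0.
; A HitStop macro briefly changes an actor's CustomTimeDilation, then restores it to normal after a delay.
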(fn `InitializeStatus`
  (params (ID :type Integer))
  (locals (NewLocalVar_0 :type " Structure"))
  (bind _outrownames (`DataTableFunctionLibrary.GetDataTableRowNames` "/Game/Character/CharacterData.CharacterData"))
  (for (_array_element _array_index) _outrownames
    (if (== _array_index ID)
      (bind _returnvalue (`|GetDataTableRow` "/Game/Character/CharacterData.CharacterData" _array_element)
        (:`then`
          (set `self.HP` (`.MaxHP` (break `MyData` _returnvalue)))
          (set `self.MyParam` (make `CharacterStatus` (break `MyData` _returnvalue) (`.Name` (break `MyData` _returnvalue)) (`.MaxHP` (break `MyData` _returnvalue)) (`.Power` (break `MyData` _returnvalue)) (`.Defence` (break `MyData` _returnvalue)))))))))

(fn `InputInitialize`
  (bind _returnvalue (`DirectInputPadFunctionLibrary.GetDirectInputPadJoystick` 0))
  (`DirectInputPadJoystick.SetKeyMap` _returnvalue "XIGamePad_Button_A" "DIGamePad_Button2" false)
  (`DirectInputPadJoystick.SetKeyMap` _returnvalue "XIGamePad_Button_B" "DIGamePad_Button3" false))

(fn `UserConstructionScript`)