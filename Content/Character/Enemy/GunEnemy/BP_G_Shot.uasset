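; Projectile fired by gun enemies that damages the sword character on contact.
; On BeginPlay it launches along its owner's forward vector at a fixed speed and caches that owner as a BP_GunEnemyBase.
; When its collision sphere overlaps a BP_SwordCharacter, it delegates damage to the owner's GiveDamage, passing the target's Defence, then destroys itself.
; Overlaps with other actors are ignored.
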(event `self.ReceiveBeginPlay`
  (bind _returnvalue (`self.GetOwner`))
  (set `MovementComponent.Velocity` (* (`self.GetActorForwardVector` _returnvalue) 1000.0) (`self.ProjectileMovement`))
  (bind _asbp_gun_enemy_base (cast `/Game/Character/Enemy/GunEnemy/BP_GunEnemyBase` _returnvalue))
  (set `self.MyCharacter` _asbp_gun_enemy_base))

(event `self.SphereCollision.OnComponentBeginOverlap`
  (params (OverlappedComponent :type "PrimitiveComponent Object Reference") (OtherActor :type "Actor Object Reference") (OtherComp :type "PrimitiveComponent Object Reference") (OtherBodyIndex :type Integer) (bFromSweep :type Boolean) (SweepResult :type "HitResult Structure (by ref)"))
  (bind _asbp_sword_character (cast `/Game/Character/BP_SwordCharacter` OtherActor))
  (bind (_myparam_id _myparam_name _myparam_maxhp _myparam_power _myparam_defence) (break `CharacterStatus` (`ActionGameCharacter.MyParam` _asbp_sword_character)))
  (`EnemyCharacter.GiveDamage` (`self.MyCharacter`) _asbp_sword_character _myparam_defence)
  (`self.K2_DestroyActor`))

(fn `UserConstructionScript`)