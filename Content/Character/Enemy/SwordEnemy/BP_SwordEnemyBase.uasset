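; BP_SwordEnemyBase is the base Blueprint for sword enemies, providing stat setup and a parameter UI.
; InitializeStatus finds the row matching a given name in the MyCharacterData table, then fills current HP and the parameter struct from it.
; UISwitch removes and clears the widget when passed true, or creates a UI_EnemyParam bound to this enemy when false.
; The event graph and construction script hold no logic.
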(fn `InitializeStatus`
  (params (Name :type Name))
  ;[1 1 1] ステータスの初期化
  (bind _outrownames (`DataTableFunctionLibrary.GetDataTableRowNames` "/Game/Character/MyCharacterData.MyCharacterData"))
  (for _array_element _outrownames
    (if (== _array_element Name)
      (bind _returnvalue (`|GetDataTableRow` "/Game/Character/MyCharacterData.MyCharacterData" _array_element)
        (:`then`
          (set `self.currentHP` (`.MaxHP` (break `MyData` _returnvalue)))
          (set `self.MyParam` (make `CharacterStatus` (break `MyData` _returnvalue) (`.Name` (break `MyData` _returnvalue)) (`.MaxHP` (break `MyData` _returnvalue)) (`.Power` (break `MyData` _returnvalue)) (`.Defence` (break `MyData` _returnvalue)) (`.AttackRange` (break `MyData` _returnvalue)))))))))

(fn `UI_Initialize`
  ;[1 1 1] UIの初期化
  (set `self.MyUI` null))

(fn `UI_Switch`
  (params (Value :type Boolean))
  ;[1 1 1] UIの表示切替
  (if Value
    (`Widget.RemoveFromParent` (`self.MyUI`))
    (`self.UI_Initialize`)
    (else
      (bind _returnvalue (`|CreateWidget` "/Game/Character/Enemy/Widget/UI_EnemyParam.UI_EnemyParam_C" (`GameplayStatics.GetPlayerController` 0)))
      (bind _output_get (set `self.MyUI` _returnvalue))
      (set `/Game/Character/Widget/UI_CharacterMaster.EnemyCharacter` self _output_get)
      (`UserWidget.AddToViewport` _returnvalue 0))))

(fn `UserConstructionScript`)