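; Sword enemy character that turns toward its detected target, attacks the player with two blades and ragdolls on death before being destroyed.
; BeginPlay binds anim instance and game instance events for attack flow, death and UI visibility, plus combo events that toggle blade collision.
; Blade overlaps deal damage with effect, sound and hit stop via CustomTimeDilation.
; Incoming damage drains HP through a timeline; non-lethal hits also clear the target.
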(event `DamageCancel`
  ;[1 1 1] イベントにバインドしていく
  ;;[1 1 1] ダメージ処理の中止
  (set `self.Damaging` (not (`self.Damaging`))))

(event `Attackcancel`
  ;[1 1 1] イベントにバインドしていく
  ;;[1 1 1] 攻撃中止
  (set `self.Attacking` false))

(event `EventBind`
  (bind _myanim (`self.MyAnim`))
  ;[1 1 1] イベントにバインドしていく
  (add `self.PlayerCombo` (delegate `SetCollision`))
  (add `self.CollisionEnd` (delegate `SetUnCollision`))
  (add `self.OnHitStop` (delegate `HitStopEvent`))
  (add `/Game/GameMain/BP_ActionGameInstance.CheckPause` (`self.MyGameInstance`) (delegate `CheckUI`))
  (add `/Game/Character/Animation/SwordCharacter/Enemy/BP_EnemyAnim.CharacterDeath` _myanim (delegate `self.EnemyDeath`))
  (add `/Game/Character/Animation/SwordCharacter/Enemy/BP_EnemyAnim.AttackCancel` _myanim (delegate `Attackcancel`))
  (add `/Game/Character/Animation/SwordCharacter/Enemy/BP_EnemyAnim.Damage` _myanim (delegate `DamageCancel`))
  (add `/Game/Character/Animation/SwordCharacter/Enemy/BP_EnemyAnim.ComboEnd` _myanim (delegate `AttackEnd`)))

(event `self.ReceiveBeginPlay`
  ;[1 1 1] 初期化
  (bind _asbp_enemy_anim (cast `/Game/Character/Animation/SwordCharacter/Enemy/BP_EnemyAnim` (`SkeletalMeshComponent.GetAnimInstance` (`self.Mesh`))))
  (set `self.MyAnim` _asbp_enemy_anim)
  (`self.InitializeStatus` "S_Enemy")
  (bind _asbp_my_game_mode (cast `/Game/BP_MyGameMode` (`GameplayStatics.GetGameMode`)))
  (set `self.MyGameMode` _asbp_my_game_mode)
  (bind _asbp_action_game_instance (cast `/Game/GameMain/BP_ActionGameInstance` (`GameplayStatics.GetGameInstance`)))
  (set `self.MyGameInstance` _asbp_action_game_instance)
  (`self.EventBind`))

(event `SetCollision` :!signature `self.PlayerCombo`
  (params (Count :type Integer))
  ;[1 1 1] イベントにバインドしていく
  ;;[1 1 1] コリジョンの設定(有効化)
  (switch `int` Count
    (:`0`
      (`self.UseCollision` (`self.RightBlade`)))
    (:`1`
      (`self.UseCollision` (`self.LeftBlade`)))))

(event `HitStopEvent` :!signature `self.OnHitStop`
  (params (Delation :type "Float (double-precision)") (Interval :type "Float (double-precision)"))
  ;[1 1 1] イベントにバインドしていく
  ;;[1 1 1] ヒットストップ
  (`self.HitStop` self Delation Interval))

(event `AttackEnd`
  ;[1 1 1] イベントにバインドしていく
  ;;[1 1 1] 攻撃終了
  (set `self.Attacking` false)
  (`self.CollisionEnd`))

(event `SetUnCollision`
  ;[1 1 1] イベントにバインドしていく
  ;;[1 1 1] コリジョンの設定(無効化)
  (`self.UnUseCollision` (`self.LeftBlade`) (`self.RightBlade`)))

(event `self.EnemyDeath`
  ;[1 1 1] イベントにバインドしていく
  ;;[1 1 1] 死亡処理
  (`SkeletalMeshComponent.SetAllBodiesSimulatePhysics` (`self.Mesh`) true)
  (`PrimitiveComponent.SetCollisionEnabled` (`self.Mesh`) "NoCollision")
  (`KismetSystemLibrary.Delay` 1.0)
  (`/Game/GameMain/BP_ActionGameInstance.CountEvent` (`self.MyGameInstance`) false)
  (`Widget.RemoveFromParent` (`self.MyUI`))
  (`self.K2_DestroyActor`))

(event `CheckUI`
  (params (Value :type Boolean))
  ;[1 1 1] イベントにバインドしていく
  ;;[1 1 1] UIの表示非表示
  (`self.UI_Switch` Value))

(event `self.EnemyAction`
  ;[1 1 1] 攻撃イベント
  (if (not (and (`self.Attacking`) (not (`self.IsDeath`))))
    (`/Game/Character/Animation/SwordCharacter/Enemy/BP_EnemyAnim.AttackEvent` (`self.MyAnim`))
    (set `self.Attacking` true)))

(event `self.ReceiveTick`
  (params (DeltaSeconds :type "Float (single-precision)"))
  (bind _targetactor (`self.TargetActor`))
  (bind _myui (`self.MyUI`))
  (bind (_returnvalue_roll _returnvalue_pitch _returnvalue_yaw) (`KismetMathLibrary.BreakRotator` (`KismetMathLibrary.RInterpTo` (`self.K2_GetActorRotation`) (`KismetMathLibrary.FindLookAtRotation` (`self.K2_GetActorLocation`) (`self.K2_GetActorLocation` _targetactor)) (`GameplayStatics.GetWorldDeltaSeconds`) 3.0)))
  ;[1 1 1] 更新処理
  (`|ExecutionSequence`
    (:`then_0`
      ;;[1 1 1] UIの表示
      (if (`KismetSystemLibrary.IsValid` _myui)
        (`/Game/Character/Widget/UI_CharacterMaster.SetUIPosition` _myui false)))
    (:`then_1`
      (if (and (`self.IsSerch`) (`KismetSystemLibrary.IsValid` _targetactor))
        (`self.K2_SetActorRotation` (`KismetMathLibrary.MakeRotator` 0.0 0.0 _returnvalue_yaw))))))

(event `self.RightBlade.OnComponentBeginOverlap`
  (params (OverlappedComponent :type "PrimitiveComponent Object Reference") (OtherActor :type "Actor Object Reference") (OtherComp :type "PrimitiveComponent Object Reference") (OtherBodyIndex :type Integer) (bFromSweep :type Boolean) (SweepResult :type "HitResult Structure (by ref)"))
  ;[1 1 1] 攻撃判定
  (bind _asbp_sword_character (cast `/Game/Character/Player/BP_SwordCharacter` OtherActor))
  (bind (_myparam_id _myparam_name _myparam_maxhp _myparam_power _myparam_defence) (break `CharacterStatus` (`ActionGameCharacter.MyParam` _asbp_sword_character)))
  (`self.GiveDamage` _asbp_sword_character _myparam_defence)
  (bind _returnvalue (`|SpawnActorFromClass` "/Game/Character/Effect/BP_AttackEffect_01.BP_AttackEffect_01_C" (`SceneComponent.K2_GetComponentToWorld` OverlappedComponent) "Undefined" "OverrideRootScale" null null))
  (if (not (`/Game/BP_MyGameMode.GameEndFlg` (`self.MyGameMode`)))
    (`/Game/Character/Player/BP_SwordCharacter.OnHitStop` _asbp_sword_character 0.5 0.25)
    (`GameplayStatics.PlaySound2D` "/Game/Sound/SE/damage_001_Cue.Damage_001_Cue" 1.0 1.0 0.0 null null)
    (`self.HitStop` _returnvalue 0.5 0.25)))

(event `self.LeftBlade.OnComponentBeginOverlap`
  (params (OverlappedComponent :type "PrimitiveComponent Object Reference") (OtherActor :type "Actor Object Reference") (OtherComp :type "PrimitiveComponent Object Reference") (OtherBodyIndex :type Integer) (bFromSweep :type Boolean) (SweepResult :type "HitResult Structure (by ref)"))
  ;[1 1 1] 攻撃判定
  (bind _asbp_sword_character (cast `/Game/Character/Player/BP_SwordCharacter` OtherActor))
  (bind (_myparam_id _myparam_name _myparam_maxhp _myparam_power _myparam_defence) (break `CharacterStatus` (`ActionGameCharacter.MyParam` _asbp_sword_character)))
  (`self.GiveDamage` _asbp_sword_character _myparam_defence)
  (bind _returnvalue (`|SpawnActorFromClass` "/Game/Character/Effect/BP_AttackEffect_01.BP_AttackEffect_01_C" (`SceneComponent.K2_GetComponentToWorld` OverlappedComponent) "Undefined" "OverrideRootScale" null null))
  (if (not (`/Game/BP_MyGameMode.GameEndFlg` (`self.MyGameMode`)))
    (`/Game/Character/Player/BP_SwordCharacter.OnHitStop` _asbp_sword_character 0.5 0.25)
    (`GameplayStatics.PlaySound2D` "/Game/Sound/SE/damage_001_Cue.Damage_001_Cue" 1.0 1.0 0.0 null null)
    (`self.HitStop` _returnvalue 0.5 0.25)))

(event `self.BeginSerch`
  (params (_actor :type "Actor Object Reference"))
  ;[1 1 1] 索敵状態の管理
  (`self.SerchTarget` _actor true))

(event `self.SerchLost`
  ;[1 1 1] 索敵状態の管理
  (`self.SerchTarget` null))

(event `self.ReceiveAnyDamage`
  (params (Damage :type "Float (single-precision)") (DamageType :type "DamageType Object Reference") (InstigatedBy :type "Controller Object Reference") (DamageCauser :type "Actor Object Reference"))
  (bind _myanim (`self.MyAnim`))
  (bind _returnvalue (- (`self.TotalDamage`) Damage))
  ;[1 1 1] ダメージ処理
  (bind _output_get (set `self.TotalDamage` (`self.currentHP`)))
  (if (<= _returnvalue 0.0)
    (bind (_direction _deltatime) (`Timeline|DamageValue` :!via `PlayFromStart` :!label _label)
      (:`Update`
        (bind _output_get_2 (set `self.currentHP` (`KismetMathLibrary.Lerp` _output_get _returnvalue _deltatime)))
        (if (<= _output_get_2 0.0)
          (`/Engine/EditorBlueprintResources/StandardMacros.DoOnce` false
            (:`Completed`
              (set `self.IsDeath` true)
              (`/Game/Character/Animation/SwordCharacter/Enemy/BP_EnemyAnim.ComboCancel` _myanim)
              (`/Game/Character/Animation/SwordCharacter/Enemy/BP_EnemyAnim.DeathEvent` _myanim))))))
    (else
      (`/Game/Character/Animation/SwordCharacter/Enemy/BP_EnemyAnim.DamageEvent` (`self.MyAnim`))
      (`self.SerchLost`)
      (goto _label :!via `PlayFromStart`))))

(fn `UserConstructionScript`
  (`parent.UserConstructionScript`))