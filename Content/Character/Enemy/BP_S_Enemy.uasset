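; Dual-blade enemy character Blueprint that attacks the sword player, shows a screen-tracking parameter widget and handles its own damage.
; Anim combo-end and combo events drive attack state and toggle per-blade collision boxes.
; Blade overlaps deal defence-aware damage and spawn effects, with hit stop via brief CustomTimeDilation on enemy and effect.
; Incoming damage lerps HP through a timeline, playing a reaction or removing widget and actor at zero.
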(event `self.ReceiveBeginPlay`
  ;[1 1 1] 初期化
  (bind _asbp_enemy_anim (cast `/Game/Character/Animation/SwordCharacter/Enemy/BP_EnemyAnim` (`SkeletalMeshComponent.GetAnimInstance` (`self.Mesh`))))
  (bind _output_get (set `self.MyAnim` _asbp_enemy_anim))
  (add `/Game/Character/Animation/SwordCharacter/Enemy/BP_EnemyAnim.ComboEnd` _output_get (delegate `AttackEnd`))
  (add `self.PlayerCombo` (delegate `SetCollision`))
  (add `self.CollisionEnd` (delegate `SetUnCollision`))
  (add `self.E_HitStop` (delegate `HitStopEvent`))
  (`self.InitializeStatus` 1)
  (bind _returnvalue (`|CreateWidget` "/Game/Character/Enemy/Widget/UI_EnemyParam.UI_EnemyParam_C" (`GameplayStatics.GetPlayerController` 0)))
  (bind _output_get_2 (set `self.MyUI` _returnvalue))
  (set `/Game/Character/Widget/UI_CharacterMaster.MyCharacter` self _output_get_2)
  (`UserWidget.AddToViewport` _returnvalue 0))

(event `AttackEnd`
  ;[1 1 1] 攻撃終了
  (set `self.Attacking` false)
  (`self.CollisionEnd`))

(event `HitStopEvent`
  ;[1 1 1] ヒットストップ
  (`self.HitStop` self 0.5 0.25))

(event `self.ReceiveTick`
  (params (DeltaSeconds :type "Float (single-precision)"))
  (bind _myui (`self.MyUI`))
  (if (`KismetSystemLibrary.IsValid` _myui)
    (`/Game/Character/Widget/UI_CharacterMaster.SetUIPosition` _myui)))

(event `SetUnCollision`
  ;[1 1 1] コリジョンの設定(無効化)
  (`self.UnUseCollision` (`self.LeftBlade`) (`self.RightBlade`)))

(event `SetCollision` :!signature `self.PlayerCombo`
  (params (Count :type Integer))
  ;[1 1 1] コリジョンの設定(有効化)
  (switch `int` Count
    (:`0`
      (`self.UseCollision` (`self.RightBlade`)))
    (:`1`
      (`self.UseCollision` (`self.LeftBlade`)))))

(event `EnemyAttack`
  ;[1 1 1] 攻撃イベント
  (if (not (`self.Attacking`))
    (`/Game/Character/Animation/SwordCharacter/Enemy/BP_EnemyAnim.AttackEvent` (`self.MyAnim`))
    (set `self.Attacking` true)))

(event `self.RightBlade.OnComponentBeginOverlap`
  (params (OverlappedComponent :type "PrimitiveComponent Object Reference") (OtherActor :type "Actor Object Reference") (OtherComp :type "PrimitiveComponent Object Reference") (OtherBodyIndex :type Integer) (bFromSweep :type Boolean) (SweepResult :type "HitResult Structure (by ref)"))
  ;[1 1 1] 攻撃判定
  (bind _asbp_sword_character (cast `/Game/Character/BP_SwordCharacter` OtherActor))
  (bind (_myparam_id _myparam_name _myparam_maxhp _myparam_power _myparam_defence) (break `CharacterStatus` (`ActionGameCharacter.MyParam` _asbp_sword_character)))
  (`self.GiveDamage` _asbp_sword_character _myparam_defence)
  (bind _returnvalue (`|SpawnActorFromClass` "/Game/Effect/BP_AttackEffect.BP_AttackEffect_C" (`SceneComponent.K2_GetComponentToWorld` OverlappedComponent) "Undefined" "OverrideRootScale" null null))
  (`self.E_HitStop`)
  (`self.HitStop` _returnvalue 0.5 0.25))

(event `self.LeftBlade.OnComponentBeginOverlap`
  (params (OverlappedComponent :type "PrimitiveComponent Object Reference") (OtherActor :type "Actor Object Reference") (OtherComp :type "PrimitiveComponent Object Reference") (OtherBodyIndex :type Integer) (bFromSweep :type Boolean) (SweepResult :type "HitResult Structure (by ref)"))
  ;[1 1 1] 攻撃判定
  (bind _asbp_sword_character (cast `/Game/Character/BP_SwordCharacter` OtherActor))
  (bind (_myparam_id _myparam_name _myparam_maxhp _myparam_power _myparam_defence) (break `CharacterStatus` (`ActionGameCharacter.MyParam` _asbp_sword_character)))
  (`self.GiveDamage` _asbp_sword_character _myparam_defence)
  (bind _returnvalue (`|SpawnActorFromClass` "/Game/Effect/BP_AttackEffect.BP_AttackEffect_C" (`SceneComponent.K2_GetComponentToWorld` OverlappedComponent) "Undefined" "OverrideRootScale" null null))
  (`self.E_HitStop`)
  (`self.HitStop` _returnvalue 0.5 0.25))

(event `self.ReceiveAnyDamage`
  (params (Damage :type "Float (single-precision)") (DamageType :type "DamageType Object Reference") (InstigatedBy :type "Controller Object Reference") (DamageCauser :type "Actor Object Reference"))
  (bind _returnvalue (- (`self.TotalDamage`) Damage))
  ;[1 1 1] ダメージ処理
  (bind _output_get (set `self.TotalDamage` (`self.HP`)))
  (if (<= _returnvalue 0.0)
    (bind (_direction _deltatime) (`Timeline|DamageValue` :!via `PlayFromStart` :!label _label)
      (:`Update`
        (bind _output_get_2 (set `self.HP` (`KismetMathLibrary.Lerp` _output_get _returnvalue _deltatime)))
        (if (<= _output_get_2 0.0)
          (`Widget.RemoveFromParent` (`self.MyUI`))
          (`self.K2_DestroyActor`))))
    (else
      (`/Game/Character/Animation/SwordCharacter/Enemy/BP_EnemyAnim.DamageEvent` (`self.MyAnim`))
      (goto _label :!via `PlayFromStart`))))

(fn `UserConstructionScript`
  (`parent.UserConstructionScript`))