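; Rampage boss enemy character that attacks the player, shows a boss parameter widget and ragdolls on death.
; AI controller events trigger weak, combo, quake and delay actions on the anim instance.
; Anim events return to toggle left/right hit colliders that damage the player, shake the camera and end attacks.
; Damage lerps HP through a timeline, firing the death animation once at zero.
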(event `CameraShake`
  ;[1 1 1] カメラ振動
  (`PlayerController.ClientStartCameraShake` :`self` (`GameplayStatics.GetPlayerController` 0) :`Shake` "/Game/Character/Enemy/BossEnemy/BP_CameraShake.BP_CameraShake_C"))

(event `self.ReceiveBeginPlay`
  ;[1 1 1] 初期化
  (bind _asbp_rampage_anim (cast `/Game/Character/Animation/BossEnemy/BP_RampageAnim` (`SkeletalMeshComponent.GetAnimInstance` (`self.Mesh`))))
  (set `self.MyAnim` _asbp_rampage_anim)
  (bind _asaic_boss_enemy_controller_base (cast `/Game/Character/Enemy/AIController/AIC_BossEnemyControllerBase` (`self.GetController`)))
  (set `self.MyController` _asaic_boss_enemy_controller_base)
  (`self.EventBind`)
  (`self.InitializeStatus` "Boss")
  (bind _returnvalue (`|CreateWidget` "/Game/Character/Enemy/Widget/UI_BossPAram.UI_BossParam_C"))
  (set `/Game/Character/Enemy/Widget/UI_BossPAram.MyCharacter` self _returnvalue)
  (`UserWidget.AddToViewport` _returnvalue 0)
  (bind _asbp_my_game_mode (cast `/Game/BP_MyGameMode` (`GameplayStatics.GetGameMode`)))
  (`/Game/GameMain/Widget/UI_Master.CreateChild` (`/Game/BP_MyGameMode.UI_Main` _asbp_my_game_mode) _returnvalue 1))

(event `EventBind`
  (bind _mycontroller (`self.MyController`))
  (bind _myanim (`self.MyAnim`))
  ;[1 1 1] イベントにバインドする
  (add `/Game/Character/Animation/BossEnemy/BP_RampageAnim.CollisionStart` _myanim (delegate `CollisionStart`))
  (add `/Game/Character/Animation/BossEnemy/BP_RampageAnim.CollisionEnd` _myanim (delegate `CollisionEnd`))
  (add `/Game/Character/Animation/BossEnemy/BP_RampageAnim.AttackEnd` _myanim (delegate `AttackEnd`))
  (add `/Game/Character/Animation/BossEnemy/BP_RampageAnim.BossDeath` _myanim (delegate `BossDeath`))
  (add `/Game/Character/Animation/BossEnemy/BP_RampageAnim.QuakeStart` _myanim (delegate `CameraShake`))
  (add `/Game/Character/Enemy/AIController/AIC_BossEnemyControllerBase.WeakAttack` _mycontroller (delegate `WeakAttack`))
  (add `/Game/Character/Enemy/AIController/AIC_BossEnemyControllerBase.ComboAttack` _mycontroller (delegate `ComboAttack`))
  (add `/Game/Character/Enemy/AIController/AIC_BossEnemyControllerBase.Quake` _mycontroller (delegate `QuakeAction`))
  (add `/Game/Character/Enemy/AIController/AIC_BossEnemyControllerBase.BossDelay` _mycontroller (delegate `BossDelay`)))

(event `CollisionStart`
  (params (ColName :type Name))
  ;[1 1 1] イベントにバインドする
  ;;[1 1 1] 当たり判定の有効化
  (switch `name` ColName
    (:`Right`
      (`self.UseCollision` (`self.RightCol`)))
    (:`Left`
      (`self.UseCollision` (`self.LeftCol`)))))

(event `CollisionEnd`
  ;[1 1 1] イベントにバインドする
  ;;[1 1 1] 当たり判定の無効化
  (`self.UnUseCollision` (`self.RightCol`) (`self.LeftCol`)))

(event `BossDeath`
  (bind _mesh (`self.Mesh`))
  ;[1 1 1] イベントにバインドする
  ;;[1 1 1] 死亡処理
  (`SkeletalMeshComponent.SetAllBodiesSimulatePhysics` _mesh true)
  (`PrimitiveComponent.SetCollisionEnabled` _mesh "PhysicsOnly")
  (`PrimitiveComponent.SetCollisionEnabled` (`self.CapsuleComponent`) "NoCollision")
  (`self.CollisionEnd`))

(event `WeakAttack`
  ;[1 1 1] イベントにバインドする
  ;;[1 1 1] 弱攻撃
  (set `self.Attacking` true)
  (`/Game/Character/Animation/BossEnemy/BP_RampageAnim.WeakAttack` (`self.MyAnim`)))

(event `ComboAttack`
  ;[1 1 1] イベントにバインドする
  ;;[1 1 1] コンボ攻撃
  (set `self.Attacking` true)
  (`/Game/Character/Animation/BossEnemy/BP_RampageAnim.ComboAttack` (`self.MyAnim`)))

(event `QuakeAction`
  ;[1 1 1] イベントにバインドする
  ;;[1 1 1] 衝撃攻撃
  (set `self.Attacking` true)
  (`/Game/Character/Animation/BossEnemy/BP_RampageAnim.QuakeAttack` (`self.MyAnim`)))

(event `BossDelay`
  ;[1 1 1] イベントにバインドする
  ;;[1 1 1] 隙を見せる
  (set `self.Attacking` true)
  (`/Game/Character/Animation/BossEnemy/BP_RampageAnim.BossDelay` (`self.MyAnim`)))

(event `AttackEnd`
  ;[1 1 1] イベントにバインドする
  ;;[1 1 1] 攻撃終了
  (set `self.Attacking` false))

(event `self.BeginSerch`
  (params (_actor :type "Actor Object Reference"))
  ;[1 1 1] 索敵開始
  (`self.SerchTarget` _actor true))

(event `self.RightCol.OnComponentBeginOverlap`
  (params (OverlappedComponent :type "PrimitiveComponent Object Reference") (OtherActor :type "Actor Object Reference") (OtherComp :type "PrimitiveComponent Object Reference") (OtherBodyIndex :type Integer) (bFromSweep :type Boolean) (SweepResult :type "HitResult Structure (by ref)"))
  (bind _asbp_player_character (cast `/Game/Character/Player/BP_PlayerCharacter` OtherActor))
  (bind (_myparam_id _myparam_name _myparam_maxhp _myparam_power _myparam_defence) (break `CharacterStatus` (`ActionGameCharacter.MyParam` _asbp_player_character)))
  (`self.GiveDamage` _asbp_player_character _myparam_defence))

(event `self.LeftCol.OnComponentBeginOverlap`
  (params (OverlappedComponent :type "PrimitiveComponent Object Reference") (OtherActor :type "Actor Object Reference") (OtherComp :type "PrimitiveComponent Object Reference") (OtherBodyIndex :type Integer) (bFromSweep :type Boolean) (SweepResult :type "HitResult Structure (by ref)"))
  (bind _asbp_player_character (cast `/Game/Character/Player/BP_PlayerCharacter` OtherActor))
  (bind (_myparam_id _myparam_name _myparam_maxhp _myparam_power _myparam_defence) (break `CharacterStatus` (`ActionGameCharacter.MyParam` _asbp_player_character)))
  (`self.GiveDamage` _asbp_player_character _myparam_defence))

(event `self.ReceiveAnyDamage`
  (params (Damage :type "Float (single-precision)") (DamageType :type "DamageType Object Reference") (InstigatedBy :type "Controller Object Reference") (DamageCauser :type "Actor Object Reference"))
  (bind _returnvalue (- (`self.TotalDamage`) Damage))
  ;[1 1 1] ダメージ処理
  (bind _output_get (set `self.TotalDamage` (`self.CurrentHP`)))
  (if (<= _returnvalue 0.0)
    (bind (_direction _deltatime) (`Timeline|タイムライン_0` :!via `PlayFromStart` :!label _label)
      (:`Update`
        (bind _output_get_2 (set `self.CurrentHP` (`KismetMathLibrary.Lerp` _output_get _returnvalue _deltatime)))
        (if (<= _output_get_2 0.0)
          (`/Engine/EditorBlueprintResources/StandardMacros.DoOnce` false
            (:`Completed`
              (set `self.IsDeath` true)
              (`/Game/Character/Animation/BossEnemy/BP_RampageAnim.DeathEvent` (`self.MyAnim`)))))))
    (else
      (goto _label :!via `PlayFromStart`))))

(fn `UserConstructionScript`
  (`parent.UserConstructionScript`))