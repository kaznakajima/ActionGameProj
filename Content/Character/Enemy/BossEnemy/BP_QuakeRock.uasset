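; BP_QuakeRock is a destructible rock in the boss enemy's folder that damages an action game character it hits.
; On hit, it has its owner apply damage using the character's Defence parameter, then plays a damage sound unless the game mode flags the game as ended.
; When the Destructible component fractures, it stops colliding with pawns and destroys itself after a short delay.
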(event `self.ReceiveBeginPlay`)

(event `self.Destructible.OnComponentFracture`
  (params (HitPoint :type "Vector Structure (by ref)") (HitDirection :type "Vector Structure (by ref)"))
  (`PrimitiveComponent.SetCollisionResponseToChannel` (`self.Destructible`) "ECC_Pawn" "ECR_Ignore")
  (`KismetSystemLibrary.Delay` 5.0)
  (`self.K2_DestroyActor`))

(event `self.Destructible.OnComponentHit`
  (params (HitComponent :type "PrimitiveComponent Object Reference") (OtherActor :type "Actor Object Reference") (OtherComp :type "PrimitiveComponent Object Reference") (NormalImpulse :type "Vector Structure") (Hit :type "HitResult Structure (by ref)"))
  (bind _asaction_game_character (cast `ActionGameCharacter` OtherActor))
  (bind (_myparam_id _myparam_name _myparam_maxhp _myparam_power _myparam_defence) (break `CharacterStatus` (`ActionGameCharacter.MyParam` _asaction_game_character)))
  (`BossCharacter.GiveDamage` (`self.MyOwner`) _asaction_game_character _myparam_defence)
  (bind _asbp_my_game_mode (cast `/Game/BP_MyGameMode` (`GameplayStatics.GetGameMode`)))
  (if (not (`/Game/BP_MyGameMode.GameEndFlg` _asbp_my_game_mode))
    (`GameplayStatics.PlaySound2D` "/Game/Sound/SE/damage_001_Cue.Damage_001_Cue" 1.0 1.0 0.0 null null)))

(fn `UserConstructionScript`)