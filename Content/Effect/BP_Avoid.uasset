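; BP_Avoid is a short-lived effect actor that fades its mesh through a timeline and destroys itself when the timeline finishes.
; The construction script creates a dynamic M_Avoid material, whose Alpha parameter is driven by the timeline curve multiplied by Opacity.
; SetOpacity lowers Opacity in proportion to the actor's distance from a given origin when within a fixed radius, so closer instances appear more transparent.
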(event `self.ReceiveBeginPlay`
  (bind _asmaterial_instance_dynamic (cast `MaterialInstanceDynamic` (`PrimitiveComponent.GetMaterial` (`self.Mesh`) 0)))
  (set `self.MaterialInstance` _asmaterial_instance_dynamic)
  (bind (_direction _alpha) (`Timeline|Alpha` :!via `PlayFromStart`)
    (:`Update`
      (`MaterialInstanceDynamic.SetScalarParameterValue` (`self.MaterialInstance`) "Alpha" (* _alpha (`self.Opacity`))))
    (:`Finished`
      (`self.K2_DestroyActor`))))

(fn `SetOpacity`
  (params (Origin :type "Vector Structure"))
  (bind _returnvalue (`KismetMathLibrary.VSize` (- Origin (`self.K2_GetActorLocation`))))
  (bind _returnvalue_2 (/ _returnvalue 550.0))
  (if (< _returnvalue 550.0)
    (set `self.Opacity` _returnvalue_2)
    (`MaterialInstanceDynamic.SetScalarParameterValue` (`self.MaterialInstance`) "Alpha" _returnvalue_2)))

(fn `UserConstructionScript`
  (`PrimitiveComponent.CreateDynamicMaterialInstance` (`self.Mesh`) 0 "/Game/Character/Player/Material/M_Avoid.M_Avoid" "None"))