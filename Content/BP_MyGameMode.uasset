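; Game mode that runs an action level from opening fade through boss battle to game-over or clear result.
; It tracks enemy count through GameInstance events; when none remain, a fade-out triggers the BossSpawn sequence and boss battle call.
; UI fade callbacks toggle active and pause state, and game end shows a result widget with a timeline-driven noise material.
; BGM fades via sound mix override; SpawnBossEnemy provides an AI boss spawn.
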(event `EventBind`
  (bind _ui_fade (`self.UI_Fade`))
  (bind _mygameinstance (`self.MyGameInstance`))
  ;[1 1 1] イベントにバインドしていく
  (add `/Game/GameMain/BP_ActionGameInstance.CountEvent` _mygameinstance (delegate `CountEvent`))
  (add `/Game/GameMain/BP_ActionGameInstance.GameEndEvent` _mygameinstance (delegate `GameEnd`))
  (add `/Game/GameMain/Widget/UI_Fade.FadeInEnd` _ui_fade (delegate `FadeInEvent`))
  (add `/Game/GameMain/Widget/UI_Fade.FadeOutEnd` _ui_fade (delegate `FadeOutEvent`)))

(event `self.ReceiveBeginPlay`
  ;[1 1 1] 初期化
  (bind _asbp_action_game_instance (cast `/Game/GameMain/BP_ActionGameInstance` (`GameplayStatics.GetGameInstance`)))
  (set `self.MyGameInstance` _asbp_action_game_instance)
  (bind _returnvalue (`|CreateWidget` "/Game/GameMain/Widget/UI_Master.UI_Master_C"))
  (bind _output_get (set `self.UI_Main` _returnvalue))
  (`UserWidget.AddToViewport` _output_get 0)
  (`self.PlayFade`
    (:`Output`
      (`GameplayStatics.PlaySound2D` "/Game/MegaGameMusicCollection/RockMusicPack/Cues/Fight_Till_Dying_looped_Cue.Fight_Till_Dying_looped_Cue" 1.0 1.0 0.0 null null)
      (`self.EventBind`)
      (`self.FadeStart` true)
      (`self.AllEnemyCount`))))

(event `CountEvent`
  (params (Increment :type Boolean))
  ;[1 1 1] イベントにバインドしていく
  ;;[1 1 1] エネミーの数のカウント
  (if Increment
    (`self.EnemyCountIncrement`)
    (else
      (`self.EnemyCountDecrement`))))

(event `FadeInEvent`
  (bind _mygameinstance (`self.MyGameInstance`))
  ;[1 1 1] イベントにバインドしていく
  ;;[1 1 1] フォードイン修了処理
  (if (`self.IsActive`)
    (set `/Game/GameMain/BP_ActionGameInstance.IsActive` true _mygameinstance)
    (`/Game/GameMain/BP_ActionGameInstance.CheckPause` _mygameinstance false)))

(event `FadeOutEvent`
  ;[1 1 1] イベントにバインドしていく
  ;;[1 1 1] フェードアウト終了処理
  (if (not (`self.GameEndFlg`))
    (`/Game/GameMain/BP_ActionGameInstance.CheckPause` (`self.MyGameInstance`) true)
    (bind (_outactor _returnvalue) (`LevelSequencePlayer.CreateLevelSequencePlayer` "/Game/Sequencer/BossSpawn.BossSpawn"))
    (`MovieSceneSequencePlayer.Play` _returnvalue)
    (`/Game/GameMain/Widget/UI_Fade.FadeInAnim` (`self.UI_Fade`))
    (`self.BossBattle`)
    (set `self.IsActive` false)))

(event `FadeStart`
  (params (FadeIn :type Boolean))
  (bind _mygameinstance (`self.MyGameInstance`))
  ;[1 1 1] 音量のフェード
  (if FadeIn
    (bind (_direction _volume) (`Timeline|VolumeFade` :!via `PlayFromStart` :!label _label)
      (:`Update`
        (if (<= _volume (`/Game/GameMain/BP_ActionGameInstance.B_Volume` (`self.MyGameInstance`)))
          (`GameplayStatics.SetSoundMixClassOverride` "/Game/Sound/MixMaster.MixMaster" "/Game/Sound/BGM.BGM" _volume 1.0 0.0)
          (`GameplayStatics.PushSoundMixModifier` "/Game/Sound/MixMaster.MixMaster"))))
    (elif (`/Game/GameMain/BP_ActionGameInstance.IsPause` _mygameinstance)
      (`/Game/GameMain/BP_ActionGameInstance.OnPause` _mygameinstance)
      (goto _label :!via `ReverseFromEnd`)
      (else
        (goto _label :!via `ReverseFromEnd`)))))

(event `GameEnd`
  (params (Value :type Boolean))
  (bind _mygameinstance (`self.MyGameInstance`))
  ;[1 1 1] イベントにバインドしていく
  ;;[1 1 1] ゲーム終了処理
  (set `/Game/GameMain/BP_ActionGameInstance.IsActive` false _mygameinstance)
  (`/Game/GameMain/BP_ActionGameInstance.CheckPause` _mygameinstance true)
  (bind _returnvalue (`|CreateWidget` "/Game/GameMain/Widget/UI_Result.UI_Result_C"))
  (bind _output_get (set `self.UI_Result` _returnvalue))
  (set `/Game/GameMain/Widget/UI_Result.GameOverFlg` Value _output_get)
  (`/Game/GameMain/Widget/UI_Master.CreateChild` (`self.UI_Main`) _returnvalue 5)
  (bind _returnvalue_2 (`Image.GetDynamicMaterial` (`/Game/GameMain/Widget/UI_Result.GameResult` _returnvalue)))
  (bind (_direction _noise) (`Timeline|NoiseVolume` :!via `PlayFromStart`)
    (:`Update`
      (`MaterialInstanceDynamic.SetScalarParameterValue` _returnvalue_2 "Amount" _noise))
    (:`Finished`
      (set `self.GameEndFlg` true)
      (set `/Game/GameMain/Widget/UI_Result.IsActive` true (`self.UI_Result`))
      (if (not Value)
        (`self.GameClear`)))))

(fn `AllEnemyCount`
  ;[1 1 1] レベル上の敵の数を取得
  (bind _outactors (`GameplayStatics.GetAllActorsOfClass` "/Script/ActionGame.EnemyCharacter"))
  (for _ _outactors
    (bind _result (`/Engine/EditorBlueprintResources/StandardMacros.IncrementInt` (`self.EnemyCount`))
      (:`  `
        (set `self.EnemyCount` _result)))))

(fn `EnemyCountDecrement`
  ;[1 1 1] 敵の数を減算する
  (bind _result (`/Engine/EditorBlueprintResources/StandardMacros.DecrementInt` (`self.EnemyCount`))
    (:`  `
      (bind _output_get (set `self.EnemyCount` _result))
      (if (<= _output_get 0)
        (`self.PlayFade`)))))

(fn `EnemyCountIncrement`
  ;[1 1 1] 敵の数を加算する
  (bind _result (`/Engine/EditorBlueprintResources/StandardMacros.IncrementInt` (`self.EnemyCount`))
    (:`  `
      (set `self.EnemyCount` _result))))

(fn `SpawnBossEnemy`
  ;[1 1 1] ボス敵の生成
  (bind _returnvalue (`AIBlueprintHelperLibrary.SpawnAIFromClass` "/Game/Character/Enemy/BossEnemy/Rampage/BP_RampageEnemy.BP_RampageEnemy_C" "/Game/Character/Enemy/BossEnemy/BehaviourTree/BossEnemy.BossEnemy" (0.0 -7000.0 600.0)))
  (set `Pawn.AIControllerClass` "/Game/Character/Enemy/AIController/AIC_BossRampage.AIC_BossRampage_C" _returnvalue)
  (`Pawn.SpawnDefaultController` _returnvalue)
  (bind _asbp_rampage_enemy (cast `/Game/Character/Enemy/BossEnemy/Rampage/BP_RampageEnemy` _returnvalue))
  (`/Game/Character/Enemy/BossEnemy/BossEnemyBase.CharacterInitialize` _asbp_rampage_enemy))

(fn `UserConstructionScript`)