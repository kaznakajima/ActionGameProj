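; BP_ActionGameInstance manages the game's pause menu, toggling pause and relaying menu input to the menu widget.
; OnPause creates UI_Pause as a child of the game mode's UIMain and pauses the game, or unpauses, removes the widget and resets state.
; MenuIndex forwards selection changes to the widget.
; MenuAction, when the widget is active, either plays its fade or calls OnPause, depending on the selected index.
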(fn `Initialize`
  ;[1 1 1] 初期化
  (set `self.IsPause` false)
  (set `self.MainWidget` null))

(fn `MenuAction`
  (bind _mainwidget (`self.MainWidget`))
  (if (`/Game/GameMain/Widget/UI_Pause.IsActive` _mainwidget)
    (switch `int` (`/Game/GameMain/Widget/UI_Pause.Index` _mainwidget)
      (:`0`
        (`/Game/GameMain/Widget/UI_Pause.PlayFade` (`self.MainWidget`)))
      (:`1`
        (`self.OnPause`)))))

(fn `MenuIndex`
  (params (Value :type "Float (double-precision)"))
  ;[1 1 1] メニュー選択状態の変更
  (`/Game/GameMain/Widget/UI_Pause.InputIndex` (`self.MainWidget`) Value))

(fn `OnPause`
  ;[1 1 1] メニュー画面の表示非表示
  (if (`self.IsPause`)
    (`GameplayStatics.SetGamePaused` false)
    (`Widget.RemoveFromParent` (`self.MainWidget`))
    (`self.Initialize`)
    (else
      (bind _returnvalue (`|CreateWidget` "/Game/GameMain/Widget/UI_Pause.UI_Pause_C"))
      (bind _output_get (set `self.MainWidget` _returnvalue))
      (bind _asbp_my_game_mode (cast `/Game/BP_MyGameMode` (`GameplayStatics.GetGameMode`)))
      (`/Game/GameMain/Widget/UI_Master.CreateChild` (`/Game/BP_MyGameMode.UI_Main` _asbp_my_game_mode) _output_get 0)
      (bind _returnvalue_2 (`GameplayStatics.SetGamePaused` true))
      (set `self.IsPause` _returnvalue_2))))